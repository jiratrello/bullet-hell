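; BP_TargetPerson is a possessable character that switches to a HUD view with a hidden body while a player controls it.
; Player possession adds the BPW_TargetPersonUI widget and hides the mesh; unpossession reverses both if the widget exists.
; MoveRight drives yaw, while MoveForward drives pitch and also scales forward movement input applied each Tick, multiplied by Speed and delta time.
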(event `self.ReceivePossessed`
  (params (NewController :type "Controller Object Reference"))
  (if (`Controller.IsPlayerController` NewController)
    (bind _returnvalue (`|CreateWidget` "/Game/Characters/TargetPerson/BPW_TargetPersonUI.BPW_TargetPersonUI_C"))
    (bind _output_get (set `self.UI` _returnvalue))
    (`UserWidget.AddToViewport` _output_get 0)
    (`SceneComponent.SetVisibility` (`self.Mesh`) false true)))

(event `self.ReceiveUnpossessed`
  (params (OldController :type "Controller Object Reference"))
  (bind _ui (`self.UI`))
  (`/Engine/EditorBlueprintResources/StandardMacros.IsValid` _ui
    (:`Is Valid`
      (`Widget.RemoveFromParent` _ui)
      (`SceneComponent.SetVisibility` (`self.Mesh`) true true))))

(event `self.ReceiveTick`
  (params (DeltaSeconds :type "Float (single-precision)"))
  (`PawnMovementComponent.AddInputVector` (`self.CharacterMovement`) (* (* (* (`KismetMathLibrary.GetForwardVector` (`self.K2_GetActorRotation`)) (`self.GetInputAxisValue`)) DeltaSeconds) (`self.speed`)) false))

(event `InputAxis|MoveRight`
  (params (AxisValue :type "Float (single-precision)"))
  (`self.AddControllerYawInput` AxisValue))

(event `InputAxis|MoveForward`
  (params (AxisValue :type "Float (single-precision)"))
  (`self.AddControllerPitchInput` AxisValue))

(fn `UserConstructionScript`)