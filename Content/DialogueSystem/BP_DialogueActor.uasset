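; World-space NPC dialogue actor that types lines letter by letter on 3D text with looping speech audio while the player overlaps it.
; Looping timers drive typing and yaw-facing toward the player; advancing completes the line, moves on, or shows a repeat icon at the end.
; An instigator alternates turns with linked conversants through messages, checking their typer timers.
; The construction script rebuilds lines with breaks every N words.
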(event `self.ReceiveBeginPlay`
  (bind _horizontalalignment (`self.HorizontalAlignment`))
  ;[1 1 1] Setup timers and widget ref
  (bind _returnvalue (`KismetSystemLibrary.K2_SetTimer` null "WidgetFacePlayer" 0.2 true))
  (bind _output_get (set `self.FacePlayer` _returnvalue))
  (`KismetSystemLibrary.K2_PauseTimerHandle` _output_get)
  (bind _returnvalue_2 (`KismetSystemLibrary.K2_SetTimer` null "Type" (`self.TypeTIme`) true))
  (bind _output_get_2 (set `self.TyperHandler` _returnvalue_2))
  (`KismetSystemLibrary.K2_PauseTimerHandle` _output_get_2)
  (`self.ResetDialogue`)
  (set `self.HowManyConversants` (`KismetArrayLibrary.Array_LastIndex` (`self.OtherConversant`)))
  (if (`|EnumEquality` _horizontalalignment "EHTA_Left")
    (`SceneComponent.K2_SetRelativeLocation` (`self.SPR_RepeatImg_Sprite`) (0.0 -60.0 2.0) false false)
    (set `self.TextRotOffset` 10.0)
    (elif (`|EnumEquality` _horizontalalignment "EHTA_Right")
      (`SceneComponent.K2_SetRelativeLocation` (`self.SPR_RepeatImg_Sprite`) (0.0 60.0 2.0) false false)
      (set `self.TextRotOffset` -10.0)
      (else
        (`SceneComponent.K2_SetRelativeLocation` (`self.SPR_RepeatImg_Sprite`) (0.0 0.0 2.0) false false)
        (set `self.TextRotOffset` 0.0)))))

(event `ResetClosure`
  (bind _speakingspawnsound (`self.SpeakingSpawnSound`))
  ;[1 1 1] Typing function
  (goto _label :!via `Reset`))

(event `GoToNextLine`
  (bind _speakingspawnsound (`self.SpeakingSpawnSound`))
  ;[1 1 1] Typing function
  (bind _result (`/Engine/EditorBlueprintResources/StandardMacros.IncrementInt` (`self.DialogueLine`))
    (:`  `
      (if (>= _result (`KismetArrayLibrary.Array_Length` (`self.FullTextUpdated`)))
        (`/Engine/EditorBlueprintResources/StandardMacros.DoOnce` false :!label _label
          (:`Completed`
            (`KismetSystemLibrary.K2_PauseTimerHandle` (`self.TyperHandler`))
            ;;[1 1 1] convo done
            (set `self.ConvoDone` true)
            (`/Engine/EditorBlueprintResources/StandardMacros.IsValid` _speakingspawnsound
              (:`Is Valid`
                (`AudioComponent.SetPaused` _speakingspawnsound true)))))
        (else
          (`self.ResetDialogue`)
          (`self.ResetChat`)
          (`self.Type`))))))

(event `BreakTypeDisplayEverything`
  (bind _speakingspawnsound (`self.SpeakingSpawnSound`))
  ;[1 1 1] Typing function
  (`TextRenderComponent.K2_SetText` (`self.TextRender`) (`|GetArrayItem` (`self.FullTextUpdated`) (`self.DialogueLine`)))
  (`KismetSystemLibrary.K2_PauseTimerHandle` (`self.TyperHandler`) :!label _label_2)
  (`/Engine/EditorBlueprintResources/StandardMacros.IsValid` _speakingspawnsound
    (:`Is Valid`
      (`AudioComponent.SetPaused` _speakingspawnsound true))
    (:`Is Not Valid`
      _))
  (set `self.FullLineDisplayed` true))

(event `ResetChat`
  (bind _speakingspawnsound (`self.SpeakingSpawnSound`))
  ;[1 1 1] Typing function
  (goto _label_3 :!via `Reset`))

(event `Type`
  (bind _speakingspawnsound (`self.SpeakingSpawnSound`))
  ;[1 1 1] Typing function
  (`|ExecutionSequence`
    (:`then_0`
      (`/Engine/EditorBlueprintResources/StandardMacros.DoOnce` false :!label _label_3
        (:`Completed`
          (`KismetSystemLibrary.K2_UnPauseTimerHandle` (`self.TyperHandler`))
          (`/Engine/EditorBlueprintResources/StandardMacros.IsValid` _speakingspawnsound
            (:`Is Valid`
              (`AudioComponent.SetPaused` _speakingspawnsound false))
            (:`Is Not Valid`
              _))
          (set `self.FullLineDisplayed` false))))
    (:`then_1`
      (set `self.CurrentTextToType` (`KismetStringLibrary.Concat_StrStr` (`self.CurrentTextToType`) (`KismetStringLibrary.GetSubstring` (`KismetTextLibrary.Conv_TextToString` (`|GetArrayItem` (`self.FullTextUpdated`) (`self.DialogueLine`))) (`self.i`))))
      (`/Engine/EditorBlueprintResources/StandardMacros.IncrementInt` (`self.i`)
        (:`  `
          (`TextRenderComponent.K2_SetText` (`self.TextRender`) (`KismetTextLibrary.Conv_StringToText` (`self.CurrentTextToType`)))
          (if (== (`KismetStringLibrary.Len` (`KismetTextLibrary.Conv_TextToString` (`|GetArrayItem` (`self.FullTextUpdated`) (`self.DialogueLine`)))) (`self.i`))
            (goto _label_2)))))))

(event `WidgetFacePlayer`
  (bind _textrender (`self.TextRender`))
  (bind (_returnvalue_roll _returnvalue_pitch) (`KismetMathLibrary.BreakRotator` (`SceneComponent.K2_GetComponentRotation` _textrender)))
  ;[1 1 1] widget faces player
  (bind _camref (message `/Game/GunJam/Core/BPI_PlayerCharacter.GetPOV` (`GameplayStatics.GetPlayerCharacter` 0)))
  (bind (_returnvalue_roll_2 _returnvalue_pitch_2 _returnvalue_yaw) (`KismetMathLibrary.BreakRotator` (`KismetMathLibrary.FindLookAtRotation` (`SceneComponent.K2_GetComponentLocation` _textrender) (`SceneComponent.K2_GetComponentLocation` _camref))))
  (`SceneComponent.K2_SetWorldRotation` _textrender (`KismetMathLibrary.MakeRotator` _returnvalue_roll _returnvalue_pitch (+ _returnvalue_yaw (`self.TextRotOffset`))) false false))

(event `ResetDialogue`
  ;[1 1 1] Typing function
  (`TextRenderComponent.K2_SetText` (`self.TextRender`) (`self.EmptyText`))
  (set `self.CurrentTextToType` "")
  (set `self.i` 0))

(event `/Game/DialogueSystem/BPI_DialogueInterface.DialogToggledFromAnother`
  (`/Engine/EditorBlueprintResources/StandardMacros.FlipFlop`
    (:`A`
      (set `self.ControlledFromAnotherInitiated` true))
    (:`B`
      (set `self.ControlledFromAnotherInitiated` false))))

(event `/Game/DialogueSystem/BPI_DialogueInterface.ConvoReadyToReset`
  (`SceneComponent.SetVisibility` (`self.SPR_RepeatImg_Sprite`) false false))

(event `/Game/DialogueSystem/BPI_DialogueInterface.AdvanceConversation`
  (bind _speakingspawnsound (`self.SpeakingSpawnSound`))
  (bind _output (`|GetArrayItem` (`self.OtherConversant`) (`self.CurrentConversant`)))
  (bind _output_2 (`|GetArrayItem` (`self.OtherConversant`) (`self.CurrentConversant`)))
  (bind _output_3 (`|GetArrayItem` (`self.OtherConversant`) (`self.CurrentConversant`)))
  (if (`self.ConvoInstagator`)
    (if (`self.InConvoZone`)
      (if (`self.MyTurn`)
        (bind _timerhandleref (message `/Game/DialogueSystem/BPI_DialogueInterface.LineDoneCheck` _output_2))
        (if (`KismetSystemLibrary.K2_IsTimerPausedHandle` _timerhandleref)
          (if (`self.ConvoReadyToReset_0`) :!label _label_4
            (`SceneComponent.SetVisibility` (`self.SPR_RepeatImg_Sprite`) false false)
            (set `self.ConvoReadyToReset_0` false)
            (set `self.DialogueLine` 0)
            (set `self.FullLineDisplayed` false)
            (set `self.ConvoDone` false)
            (`self.ResetClosure`)
            (`KismetSystemLibrary.K2_UnPauseTimerHandle` (`self.TyperHandler`))
            (set `self.CurrentConversant` 0)
            (`/Engine/EditorBlueprintResources/StandardMacros.IsValid` _speakingspawnsound
              (:`Is Valid`
                (`AudioComponent.SetPaused` _speakingspawnsound false))
              (:`Is Not Valid`
                _))
            (if (`self.ConvoInstagator`)
              (for _array_element (`self.OtherConversant`)
                (message `/Game/DialogueSystem/BPI_DialogueInterface.ConvoReadyToReset` _array_element)))
            (elif (`self.ConvoDone`)
              (`self.ResetDialogue` :!label _label_5)
              (`SceneComponent.SetVisibility` (`self.SPR_RepeatImg_Sprite`) true false)
              (set `self.ConvoDone` false)
              (set `self.ConvoReadyToReset_0` true)
              (if (`self.ConvoInstagator`)
                (for _array_element_2 (`self.OtherConversant`)
                  (message `/Game/DialogueSystem/BPI_DialogueInterface.ResetDialogueOnConversants` _array_element_2)))
              (elif (`self.FullLineDisplayed`)
                (`self.GoToNextLine`)
                (else
                  (`self.BreakTypeDisplayEverything`)
                  (set `self.CurrentConversant` 0)
                  (set `self.MyTurn` false))))))
        (elif (`KismetSystemLibrary.K2_IsTimerPausedHandle` (`self.TyperHandler`))
          (bind _startedyet (message `/Game/DialogueSystem/BPI_DialogueInterface.SetupControlledFromAnotherCheck` _output_2))
          (if _startedyet
            (message `/Game/DialogueSystem/BPI_DialogueInterface.AdvanceConversation` _output_3)
            (else
              (message `/Game/DialogueSystem/BPI_DialogueInterface.OtherInstagatorStart` _output_3)
              ;[1 1 1] need to send to other one that it's all typed out whenever that happens
              (message `/Game/DialogueSystem/BPI_DialogueInterface.DialogToggledFromAnother` _output)))
          (bind _timerhandleref_2 (message `/Game/DialogueSystem/BPI_DialogueInterface.LineDoneCheck` _output))
          (if (`KismetSystemLibrary.K2_IsTimerPausedHandle` _timerhandleref_2)
            (bind _result (`/Engine/EditorBlueprintResources/StandardMacros.IncrementInt` (`self.CurrentConversant`))
              (:`  `
                (if (>= _result (`KismetArrayLibrary.Array_Length` (`self.OtherConversant`)))
                  (set `self.CurrentConversant` 0)
                  (set `self.MyTurn` true))))))))
    (else
      (goto _label_4))))

(event `/Game/DialogueSystem/BPI_DialogueInterface.ResetDialogueOnConversants`
  (goto _label_5))

(event `/Game/DialogueSystem/BPI_DialogueInterface.OtherInstagatorStart`
  ;[1 1 1] Activate on begin overlap
  (`SceneComponent.SetHiddenInGame` (`self.TextRender`) false false :!label _label_6)
  (`KismetSystemLibrary.K2_UnPauseTimerHandle` (`self.FacePlayer`))
  (bind _returnvalue (`GameplayStatics.SpawnSoundAtLocation` (`self.SpeakingNoise`) (`self.K2_GetActorLocation`) (struct) 1.0 1.0 0.0 null null))
  (set `self.SpeakingSpawnSound` _returnvalue)
  (`KismetSystemLibrary.K2_UnPauseTimerHandle` (`self.TyperHandler`))
  (if (== (`self.MyConversantID`) 0)
    ;;[1 1 1] other conversants wont have this ref so move convo along action won't work
    (message `/Game/GunJam/Core/BPI_PlayerCharacter.SendConvoRef` (`GameplayStatics.GetPlayerCharacter` 0) self)))

(event `self.TalkCollision.OnComponentBeginOverlap`
  (params (OverlappedComponent :type "PrimitiveComponent Object Reference") (OtherActor :type "Actor Object Reference") (OtherComp :type "PrimitiveComponent Object Reference") (OtherBodyIndex :type Integer) (bFromSweep :type Boolean) (SweepResult :type "HitResult Structure (by ref)"))
  (bind _returnvalue (`GameplayStatics.GetPlayerCharacter` 0))
  (bind _speakingspawnsound (`self.SpeakingSpawnSound`))
  (bind _charactermovement (`Character.CharacterMovement` _returnvalue))
  ;[1 1 1] Activate on begin overlap
  (if (== OtherActor _returnvalue)
    (if (not (or (`NavMovementComponent.IsFlying` _charactermovement) (`NavMovementComponent.IsFalling` _charactermovement)))
      (`/Engine/EditorBlueprintResources/StandardMacros.DoOnce` false :!label _label_7
        (:`Completed`
          (set `self.InConvoZone` true)
          (message `/Game/GunJam/Core/BPI_PlayerCharacter.InConvo` _returnvalue true)
          (`|ExecutionSequence`
            (:`then_0`
              (if (not (> (`self.MyConversantID`) 0))
                (goto _label_6)))
            (:`then_1`
              (goto _label_9 :!via `Reset`))))))))

(event `/Game/DialogueSystem/BPI_DialogueInterface.OtherInstagatorEnd`
  (bind _speakingspawnsound (`self.SpeakingSpawnSound`))
  ;[1 1 1] Deactivate on end overlap
  (`SceneComponent.SetHiddenInGame` (`self.TextRender`) true false :!label _label_8)
  (`KismetSystemLibrary.K2_PauseTimerHandle` (`self.TyperHandler`))
  (`KismetSystemLibrary.K2_PauseTimerHandle` (`self.FacePlayer`))
  (`self.ResetDialogue`)
  (set `self.DialogueLine` 0)
  (set `self.FullLineDisplayed` false)
  (set `self.ConvoDone` false)
  (`self.ResetClosure`)
  (`/Engine/EditorBlueprintResources/StandardMacros.IsValid` _speakingspawnsound
    (:`Is Valid`
      (`AudioComponent.Stop` _speakingspawnsound))
    (:`Is Not Valid`
      _))
  (`SceneComponent.SetVisibility` (`self.SPR_RepeatImg_Sprite`) false false))

(event `self.TalkCollision.OnComponentEndOverlap`
  (params (OverlappedComponent :type "PrimitiveComponent Object Reference") (OtherActor :type "Actor Object Reference") (OtherComp :type "PrimitiveComponent Object Reference") (OtherBodyIndex :type Integer))
  (bind _returnvalue (`GameplayStatics.GetPlayerCharacter` 0))
  ;[1 1 1] Deactivate on end overlap
  (if (== OtherActor _returnvalue)
    (`/Engine/EditorBlueprintResources/StandardMacros.DoOnce` false :!label _label_9
      (:`Completed`
        (set `self.InConvoZone` false)
        (message `/Game/GunJam/Core/BPI_PlayerCharacter.InConvo` _returnvalue false)
        (`|ExecutionSequence`
          (:`then_0`
            (goto _label_7 :!via `Reset`))
          (:`then_1`
            (if (> (`self.MyConversantID`) 0)
              _
              (elif (`self.ConvoInstagator`)
                (for _array_element (`self.OtherConversant`)
                  (message `/Game/DialogueSystem/BPI_DialogueInterface.OtherInstagatorEnd` _array_element)
                  (message `/Game/DialogueSystem/BPI_DialogueInterface.DialogToggledFromAnother` _array_element)
                  (`KismetSystemLibrary.PrintString` "Hello"))
                (set `self.CurrentConversant` 0)
                (set `self.MyTurn` true)
                (goto _label_8)
                (else
                  (goto _label_8))))))))))

(fn `ConvoDoneCheck`
  (returns (ConvoDone :type Boolean))
  (return (`self.ConvoDone`)))

(fn `ConvoReadyToResetCheck`
  (returns (ConvoReadyForReset :type Boolean))
  (return (`self.ConvoReadyToReset_0`)))

(fn `LineDoneCheck`
  (returns (TimerHandleRef :type "TimerHandle Structure"))
  (return (`self.TyperHandler`)))

(fn `SetupControlledFromAnotherCheck`
  (returns (StartedYet :type Boolean))
  (return (`self.ControlledFromAnotherInitiated`)))

(fn `UserConstructionScript`
  ;[1 1 1] Break the lines
  (for (_array_element _array_index) (`self.FullText`)
    (set `self.OldString` (`KismetTextLibrary.Conv_TextToString` _array_element))
    (for _index (range (+ (`KismetStringLibrary.Len` (`self.OldString`)) 1))
      (bind _returnvalue (`KismetStringLibrary.GetSubstring` (`self.OldString`) _index))
      (if (`KismetStringLibrary.EqualEqual_StrStr` _returnvalue " ")
        (bind _result (`/Engine/EditorBlueprintResources/StandardMacros.IncrementInt` (`self.WordCount`))
          (:`  `
            (if (== (mod _result (`self.InHowManySpacesBreak`)) 0)
              (bind _returnvalue_2 (`KismetStringLibrary.Concat_StrStr` (`self.NewString`) _returnvalue))
              (set `self.NewString` (`KismetStringLibrary.Concat_StrStr` _returnvalue_2 " \n"))
              (else
                (set `self.NewString` _returnvalue_2 :!label _label)))))
        (else
          (goto _label))))
    (`KismetArrayLibrary.Array_Set` (`self.FullTextUpdated`) _array_index (`KismetTextLibrary.Conv_StringToText` (`self.NewString`)) true)
    (set `self.WordCount` 0)
    (if (== _array_index 0)
      (`TextRenderComponent.K2_SetText` (`self.TextRender`) (`KismetTextLibrary.Conv_StringToText` (`self.NewString`)))
      (`TextRenderComponent.SetTextRenderColor` (`self.TextRender`) (`self.3dTextColor`))
      (`TextRenderComponent.SetHorizontalAlignment` (`self.TextRender`) (`self.HorizontalAlignment`))
      (set `self.NewString` "")
      (else
        (set `self.NewString` "")))))