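; Character Blueprint that handles mouse-look and switching between two guns.
; Weapon1 and Weapon2 inputs pass entries of the Guns class array to EquipGun, which destroys the current gun, spawns the new one and snaps it to GunSlot.
; Tick applies horizontal look as controller yaw and vertical look as clamped pitch on ViewParent, and prints a debug "character alive" message every frame.
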(event `InputAction|Weapon1`
  (params (Key :type "Key Structure"))
  (:`Pressed`
    (`self.EquipGun` (`|GetArrayItem` (`self.Guns`)))))

(event `InputAction|Trigger`
  (params (Key :type "Key Structure")))

(event `InputAction|Weapon2`
  (params (Key :type "Key Structure"))
  (:`Pressed`
    (`self.EquipGun` (`|GetArrayItem` (`self.Guns`) 1))))

(event `InputAction|Reload`
  (params (Key :type "Key Structure")))

(event `self.ReceiveBeginPlay`)

(event `self.ReceiveTick`
  (params (DeltaSeconds :type "Float (single-precision)"))
  (bind (_relativerotation_roll _relativerotation_pitch) (`KismetMathLibrary.BreakRotator` (`SceneComponent.RelativeRotation` (`self.ViewParent`))))
  (`|ExecutionSequence`
    (:`then_0`
      (`self.AddControllerYawInput` (`self.GetInputAxisValue`)))
    (:`then_1`
      (`SceneComponent.K2_SetRelativeRotation` (`self.ViewParent`) (`KismetMathLibrary.MakeRotator` 0.0 (`KismetMathLibrary.FClamp` (+ _relativerotation_pitch (`self.GetInputAxisValue`)) -90.0 90.0)) false false))
    (:`then_2`
      (`KismetSystemLibrary.PrintString` "character alive" true false (struct :`G` 0.66 :`B` 1.0 :`A` 1.0) 0.0))))

(fn `EquipGun`
  (params (Gun :type "Actor Class Reference"))
  (`|ExecutionSequence`
    (:`then_0`
      (`/Engine/EditorBlueprintResources/StandardMacros.IsValid` (`self.EquippedGun`)
        (:`Is Valid`
          (`self.K2_DestroyActor` (`self.EquippedGun`)))))
    (:`then_1`
      (bind _returnvalue (`|SpawnActorFromClass` Gun (`KismetMathLibrary.MakeTransform` (0.0 0.0 0.0)) "Undefined" "OverrideRootScale" null null))
      (bind _output_get (set `self.EquippedGun` _returnvalue))
      (`self.K2_AttachToComponent` _output_get (`self.GunSlot`) "None" "SnapToTarget" "SnapToTarget" "SnapToTarget" false))))

(fn `UserConstructionScript`)