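; Metroid-style door prop that opens when hit by an actor implementing BPI_Hittable, then closes itself after a few seconds.
; An unlocked hit switches off the point light, plays animations on front and back meshes with sound, disables box collision while open, then restores the light after closing.
; When Locked, a hit only plays an error sound; the construction script tints the light red or blue to show lock state.
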(event `self.ReceiveBeginPlay`
  (set `self.intensity` (`LightComponentBase.Intensity` (`self.PointLight`))))

(event `self.ReceiveHit`
  (params (MyComp :type "PrimitiveComponent Object Reference") (Other :type "Actor Object Reference") (OtherComp :type "PrimitiveComponent Object Reference") (bSelfMoved :type Boolean) (HitLocation :type "Vector Structure") (HitNormal :type "Vector Structure") (NormalImpulse :type "Vector Structure") (Hit :type "HitResult Structure (by ref)"))
  (if (`KismetSystemLibrary.DoesImplementInterface` Other "/Game/GunJam/Core/BPI_Hittable.BPI_Hittable_C")
    (if (`self.locked`)
      (`GameplayStatics.PlaySoundAtLocation` "/Game/GunJam/Props/MetroidDoor/incorrect_sound_effect.incorrect_sound_effect" (`self.K2_GetActorLocation`) (struct) 0.5 1.0 0.0 null null null)
      (else
        (`LightComponent.SetIntensity` (`self.PointLight`) 0.0)
        (`KismetSystemLibrary.Delay` 0.3)
        (`self.OpenDoor`)
        (`KismetSystemLibrary.Delay` 3.0)
        (`self.CloseDoor`)
        (`KismetSystemLibrary.Delay` 0.7)
        (`LightComponent.SetIntensity` (`self.PointLight`) (`self.intensity`))))))

(fn `CloseDoor`
  (`PrimitiveComponent.SetCollisionEnabled` (`self.Box`) "QueryAndPhysics")
  (`AudioComponent.SetSound` (`self.Audio`) "/Game/GunJam/Props/MetroidDoor/SW_MetroidDoor_Close.SW_MetroidDoor_Close")
  (`AudioComponent.Play` (`self.Audio`) 0.0)
  (`self.PlayAnimation` "/Game/GunJam/Props/MetroidDoor/A_MetroidDoor_Close.A_MetroidDoor_Close")
  (set `self.open` false))

(fn `OpenDoor`
  (`AudioComponent.SetSound` (`self.Audio`) "/Game/GunJam/Props/MetroidDoor/SW_MetroidDoor_Open.SW_MetroidDoor_Open")
  (`AudioComponent.Play` (`self.Audio`) 0.0)
  (`self.PlayAnimation` "/Game/GunJam/Props/MetroidDoor/A_MetroidDoor_Open.A_MetroidDoor_Open")
  (`PrimitiveComponent.SetCollisionEnabled` (`self.Box`) "NoCollision")
  (set `self.open` true))

(fn `PlayAnimation`
  (params (NewAnimToPlay :type "AnimationAsset Object Reference"))
  (`|ExecutionSequence`
    (:`then_0`
      (`SkeletalMeshComponent.PlayAnimation` (`self.Front`) NewAnimToPlay false))
    (:`then_1`
      (`SkeletalMeshComponent.PlayAnimation` (`self.Back`) NewAnimToPlay false))
    (:`then_2`
      (return))))

(fn `UserConstructionScript`
  (`LightComponent.SetLightColor` (`self.PointLight`) (`KismetMathLibrary.SelectColor` (struct :`R` 1.0 :`B` 0.01 :`A` 1.0) (struct :`R` 0.3564 :`G` 0.665387 :`B` 1.0 :`A` 1.0) (`self.locked`)) true))