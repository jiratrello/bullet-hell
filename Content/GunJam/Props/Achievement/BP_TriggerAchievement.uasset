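; BP_TriggerAchievement is a trigger actor that shows an achievement popup when the player walks into it.
; On overlap with player character 0, it creates a WBP_AchievementPopup with its TextToShow, adds it to the viewport and activates it.
; A HasFired flag makes each trigger fire only once.
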(event `self.ReceiveActorBeginOverlap`
  (params (OtherActor :type "Actor Object Reference"))
  (if (and (== OtherActor (`GameplayStatics.GetPlayerCharacter` 0)) (not (`self.HasFired`)))
    (set `self.HasFired` true)
    (bind _returnvalue (`|CreateWidget` "/Game/GunJam/Props/Achievement/WBP_AchievementPopup.WBP_AchievementPopup_C" null (`self.TextToShow`)))
    (`UserWidget.AddToViewport` _returnvalue 0)
    (`/Game/GunJam/Props/Achievement/WBP_AchievementPopup.Activate` _returnvalue)))

(fn `UserConstructionScript`)