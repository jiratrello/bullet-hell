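; BP_Target is a gun-jam target prop that shatters once when hit by an actor implementing BPI_Hittable.
; The Hit event sets a Dead flag to block repeat triggers, then after a short delay plays a pitch-randomized ding.
; It applies damage to the TargetmeshDM destructible at the hit location along the hit normal, then destroys the actor after a longer delay.
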(event `self.ReceiveHit`
  (params (MyComp :type "PrimitiveComponent Object Reference") (Other :type "Actor Object Reference") (OtherComp :type "PrimitiveComponent Object Reference") (bSelfMoved :type Boolean) (HitLocation :type "Vector Structure") (HitNormal :type "Vector Structure") (NormalImpulse :type "Vector Structure") (Hit :type "HitResult Structure (by ref)"))
  (if (not (`self.dead`))
    (if (`KismetSystemLibrary.DoesImplementInterface` Other "/Game/GunJam/Core/BPI_Hittable.BPI_Hittable_C")
      (set `self.dead` true)
      (`KismetSystemLibrary.Delay` 0.2)
      (`GameplayStatics.PlaySound2D` "/Game/GunJam/Props/Target/ding-noise-sound-effect.ding-noise-sound-effect" 1.0 (`KismetMathLibrary.RandomFloatInRange` 0.95 1.05) 0.0 null null)
      (`DestructibleComponent.ApplyDamage` (`self.Targetmesh_DM`) 10.0 HitLocation HitNormal 0.0)
      (`KismetSystemLibrary.Delay` 10.0)
      (`self.K2_DestroyActor`))))

(fn `UserConstructionScript`)