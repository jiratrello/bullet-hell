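; Base gun Blueprint that handles trigger input, ammo and equip state, leaving Fire and Reload as debug-print stubs for child classes to override.
; TryFire gates shots on ammo and a cooldown timer that Tick counts down, with Tick also repeating fire for held automatic triggers.
; SetState drives delayed Equip and Unequip transitions, and only the Active state can fire.
; TryReload refills the clip and also runs in the construction script.
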(event `Fire`
  ;[0 1 0] Abstracts, override in child classes
  (`KismetSystemLibrary.PrintString` "Fire!"))

(event `Reload`
  ;[0 1 0] Abstracts, override in child classes
  (`KismetSystemLibrary.PrintString` "Reload!"))

(event `PullTrigger`
  (set `self.bPulledTrigger` true)
  (if (`|EnumEquality` (`self.State`) "NewEnumerator1")
    (`self.TryFire`) ; (Manual firing attempt)
  ))

(event `ReleaseTrigger`
  (set `self.bPulledTrigger` false)
  (`KismetSystemLibrary.PrintString` "Released!"))

(event `self.ReceiveTick`
  (params (DeltaSeconds :type "Float (single-precision)"))
  (`|ExecutionSequence`
    (:`then_0`
      (if (> (`self.NextShotTimer`) 0.0)
        (set `self.NextShotTimer` (- (`self.NextShotTimer`) (`GameplayStatics.GetWorldDeltaSeconds`)))))
    (:`then_1`
      (if (and (`self.bPulledTrigger`) (`self.bIsAutomatic`) (`|EnumEquality` (`self.State`) "NewEnumerator1"))
        (`self.TryFire`) ; (Automatic firing attempt)
      ))
    (:`then_2`
      ;[1 1 1] Debug
      (if (`self.bDebug`)
        (`KismetSystemLibrary.PrintText` (`|FormatText` "State: {state} \nAutomatic: {auto} \nRate of Fire: {rof} \nAmmo: {ammo}" (`|GetEnumeratorNameAsString` (`self.State`)) (`self.bIsAutomatic`) (`self.RateOfFire`) (`self.Ammo`)) true false (make `LinearColor` (`KismetMathLibrary.RandomFloat`) (`KismetMathLibrary.RandomFloat`) (`KismetMathLibrary.RandomFloat`) 1.0) 0.0)))))

(event `Equip`
  (`KismetSystemLibrary.Delay` 0.5)
  (`self.SetState` "NewEnumerator1"))

(event `Unequip`
  (`KismetSystemLibrary.Delay` 0.5)
  (`self.SetState` "NewEnumerator4"))

(fn `SetState`
  (params (State :type "/Game/GunJam/Core/EGunState Enum" :default "NewEnumerator5"))
  (bind _output_get (set `self.State` State))
  (switch `/Game/GunJam/Core/EGunState` _output_get
    (:`NewEnumerator5`
      (`self.SetState` "NewEnumerator0"))
    (:`NewEnumerator0`
      (`self.Equip`))
    (:`NewEnumerator3`
      (`self.Unequip`))))

(fn `TryFire`
  (returns (OutputMessage :type String))
  (if (> (`self.Ammo`) 0)
    (if (<= (`self.NextShotTimer`) 0.0)
      (`|ExecutionSequence`
        (:`then_0`
          (set `self.NextShotTimer` (`self.RateOfFire`)))
        (:`then_1`
          (`/Engine/EditorBlueprintResources/StandardMacros.DecrementInt` (`self.Ammo`)))
        (:`then_2`
          (`self.Fire`)
          (return "Successful Fire")))
      (else
        (return "Timer less than Rate of Fire")))
    (else
      (return "Out of ammo!"))))

(fn `TryReload`
  (returns (OutputMessage :type String))
  (if (< (`self.Ammo`) (`self.ClipSize`))
    (set `self.Ammo` (`self.ClipSize`))
    (`self.Reload`)
    (return "Successful Reload")
    (else
      (return "Ammo full"))))

(fn `UserConstructionScript`
  (`self.TryReload`))