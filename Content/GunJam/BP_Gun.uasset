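; BP_Gun is a base gun Blueprint that handles trigger input, ammo and firing rate, with Fire and Reload as placeholder events for child classes to override.
; TryFire checks ammo and a cooldown timer that Tick counts down, then spends a round and calls Fire.
; Pulling the trigger fires once, and automatic guns retry every Tick while it is held.
; TryReload refills the clip and also runs in the Construction Script.
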(event `Fire`
  ;[0 1 0] Abstracts, override in child classes
  (`KismetSystemLibrary.PrintString` "Fire!"))

(event `Reload`
  ;[0 1 0] Abstracts, override in child classes
  (`KismetSystemLibrary.PrintString` "Reload!"))

(event `PullTrigger`
  (set `self.bPulledTrigger` true)
  (`self.TryFire`) ; (Manual firing attempt)
)

(event `ReleaseTrigger`
  (set `self.bPulledTrigger` false)
  (`KismetSystemLibrary.PrintString` "Released!"))

(event `self.ReceiveTick`
  (params (DeltaSeconds :type "Float (single-precision)"))
  (`|ExecutionSequence`
    (:`then_0`
      (if (> (`self.NextShotTimer`) 0.0)
        (set `self.NextShotTimer` (- (`self.NextShotTimer`) (`GameplayStatics.GetWorldDeltaSeconds`)))))
    (:`then_1`
      (if (and (`self.bPulledTrigger`) (`self.bIsAutomatic`))
        (`self.TryFire`) ; (Automatic firing attempt)
      ))
    (:`then_2`
      ;[1 1 1] Debug
      (if (`self.bDebug`)
        (`KismetSystemLibrary.PrintText` (`|FormatText` "Automatic: {auto} \nRate of Fire: {rof} \nAmmo: {ammo}" (`self.bIsAutomatic`) (`self.RateOfFire`) (`self.Ammo`)) true false (make `LinearColor` (`KismetMathLibrary.RandomFloat`) (`KismetMathLibrary.RandomFloat`) (`KismetMathLibrary.RandomFloat`) 1.0) 0.0)))))

(fn `TryFire`
  (returns (OutputMessage :type String))
  (if (> (`self.Ammo`) 0)
    (if (<= (`self.NextShotTimer`) 0.0)
      (`|ExecutionSequence`
        (:`then_0`
          (set `self.NextShotTimer` (`self.RateOfFire`)))
        (:`then_1`
          (`/Engine/EditorBlueprintResources/StandardMacros.DecrementInt` (`self.Ammo`)))
        (:`then_2`
          (`self.Fire`)
          (return "Successful Fire")))
      (else
        (return "Timer less than Rate of Fire")))
    (else
      (return "Out of ammo!"))))

(fn `TryReload`
  (returns (OutputMessage :type String))
  (if (< (`self.Ammo`) (`self.ClipSize`))
    (set `self.Ammo` (`self.ClipSize`))
    (`self.Reload`)
    (return "Successful Reload")
    (else
      (return "Ammo full"))))

(fn `UserConstructionScript`
  (`self.TryReload`))