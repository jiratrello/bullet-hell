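; Jimbo gun Blueprint that works as a treasure detector, homing in on BP_JimboTreasure actors while the trigger is held.
; Each held tick finds the nearest treasure and maps its distance to audio pitch, rising as it gets closer.
; Within close range it destroys the treasure, refreshes the list and displays a found message.
; Equip and trigger events drive the WBP_JimboUI widget and switch MediaPlayer between idle and charge sources.
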(event `self.ReceiveTick`
  (params (DeltaSeconds :type "Float (single-precision)"))
  (if (`self.held`)
    (`self.Update and Check for Treasure`)))

(event `self.Equip`
  (`MediaPlayer.OpenSource` (`self.MediaPlayer`) "/Game/Movies/IMS_JimboIdle.IMS_JimboIdle")
  (`MediaPlayer.Pause` (`self.MediaPlayer`))
  (bind _returnvalue (`|CreateWidget` "/Game/GunJam/Guns/Jimbo/WBP_JimboUI.WBP_JimboUI_C"))
  (bind _output_get (set `self.UI` _returnvalue))
  (`UserWidget.AddToViewport` _output_get 0)
  (`/Game/GunJam/Guns/Jimbo/WBP_JimboUI.Activate` (`self.UI`))
  (`self.SetState` "NewEnumerator1")
  (bind _outactors (`GameplayStatics.GetAllActorsOfClass` "/Game/GunJam/Guns/Jimbo/BP_JimboTreasure.BP_JimboTreasure_C"))
  (set `self.Treasures` _outactors))

(event `self.Unequip`
  (if (`KismetSystemLibrary.IsValid` (`self.UI`))
    (`/Game/GunJam/Guns/Jimbo/WBP_JimboUI.Unequip` (`self.UI`))
    (`KismetSystemLibrary.Delay` 0.5)
    (`Widget.RemoveFromParent` (`self.UI`)))
  (`self.SetState` "NewEnumerator4"))

(event `self.PullTrigger`
  (set `self.held` true)
  (`MediaPlayer.Play` (`self.MediaPlayer`))
  (`AudioComponent.Play` (`self.Audio`) 0.0)
  (`MediaPlayer.OpenSource` (`self.MediaPlayer`) "/Game/Movies/IMS_JimboCharge.IMS_JimboCharge")
  (`/Game/GunJam/Guns/Jimbo/WBP_JimboUI.TriggerPulled` (`self.UI`)))

(event `self.ReleaseTrigger`
  (set `self.held` false)
  (`AudioComponent.Stop` (`self.Audio`))
  (`MediaPlayer.OpenSource` (`self.MediaPlayer`) "/Game/Movies/IMS_JimboIdle.IMS_JimboIdle")
  (`/Game/GunJam/Guns/Jimbo/WBP_JimboUI.TriggerReleased` (`self.UI`)))

(fn `Get Closest Treasure`
  (returns (closestTreasure :type "/Game/GunJam/Guns/Jimbo/BP_JimboTreasure Object Reference") (distance :type "Float (double-precision)"))
  (locals (closestDistance :type "Float (double-precision)" :default 200000.0) (currentLeader :type "/Game/GunJam/Guns/Jimbo/BP_JimboTreasure Object Reference"))
  (bind _returnvalue_location (`KismetMathLibrary.BreakTransform` (`self.GetTransform`)))
  (for _array_element (`self.Treasures`)
    (bind _returnvalue_location_2 (`KismetMathLibrary.BreakTransform` (`self.GetTransform` _array_element)))
    (bind _returnvalue (`KismetMathLibrary.Vector_Distance` _returnvalue_location _returnvalue_location_2))
    (if (< _returnvalue (`local.closestDistance`))
      (set `local.currentLeader` _array_element)
      (set `local.closestDistance` _returnvalue)))
  (return (`local.currentLeader`) (`local.closestDistance`)))

(fn `Update and Check for Treasure`
  (`|ExecutionSequence`
    (:`then_0`
      (bind (_closesttreasure _distance) (`self.Get Closest Treasure`))
      (`AudioComponent.SetPitchMultiplier` (`self.Audio`) (`KismetMathLibrary.MapRangeClamped` _distance 0.0 3000.0 2.0 0.5))
      (`KismetSystemLibrary.PrintString` (`KismetStringLibrary.Conv_DoubleToString` _distance) true true (struct :`G` 0.66 :`B` 1.0 :`A` 1.0) 0.0))
    (:`then_1`
      (if (< _distance 150.0)
        (`|ExecutionSequence`
          (:`then_0`
            (set `self.held` false)
            (`AudioComponent.Stop` (`self.Audio`))
            (`self.K2_DestroyActor` _closesttreasure)
            (bind _outactors (`GameplayStatics.GetAllActorsOfClass` "/Game/GunJam/Guns/Jimbo/BP_JimboTreasure.BP_JimboTreasure_C"))
            (set `self.Treasures` _outactors))
          (:`then_1`
            (`/Game/GunJam/Guns/Jimbo/WBP_JimboUI.DisplayText` (`self.UI`) "You found it!")))))))

(fn `UserConstructionScript`
  (`parent.UserConstructionScript`))