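; RichInnerLife gun actor for the GunJam game, handling the weapon's idle animation, sway, firing feedback and equip motion.
; Procedural motion lerps the skeletal mesh around its construction-time location: mouse input drives clamped sway while Active, and firing kicks it back.
; Equip and Unequip timelines move it between holstered and initial positions, then set Active or ReadyForRemoval.
; Fire also spawns a muzzle flash and plays audio, with no hit or projectile logic here.
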(event `self.ReceiveBeginPlay`
  (`self.EnableInput` (`GameplayStatics.GetPlayerController` 0))
  (`SkeletalMeshComponent.PlayAnimation` (`self.SK_RichInnerLife`) "/Game/GunJam/Guns/RichInnerLife/A_RichInnerLife_Idle_Anim_SK_RichInnerLife_SK_RichInnerLifeAction.A_RichInnerLife_Idle_Anim_SK_RichInnerLife_SK_RichInnerLifeAction" true))

(event `InputAxisKey|MouseX` :consume false
  (params (AxisValue :type "Float (single-precision)"))
  (bind _swaymax (`self.swayMax`))
  (bind _sk_richinnerlife (`self.SK_RichInnerLife`))
  (bind _swaymax_2 (`self.swayMax`))
  (bind _returnvalue (`KismetMathLibrary.FClamp` (* AxisValue (`self.swayFactor`)) (* _swaymax -1.0) _swaymax))
  ;[1 1 1] Sway
  (switch `/Game/GunJam/Core/EGunState` (`self.State`) :!label _label
    (:`NewEnumerator1`
      (`Timeline|SwayLerpTimeline`
        (:`Update`
          (`SceneComponent.K2_SetRelativeLocation` _sk_richinnerlife (`KismetMathLibrary.VLerp` (`SceneComponent.RelativeLocation` _sk_richinnerlife) (+ (`KismetMathLibrary.MakeVector` _returnvalue _returnvalue (`KismetMathLibrary.FClamp` (/ (* (stale `InputAxisKey|MouseY` AxisValue) (`self.swayFactor`)) -1.5) (/ _swaymax_2 -2.0) (/ 0.0 _swaymax_2))) (`self.initialLocation`)) (* (`GameplayStatics.GetWorldDeltaSeconds`) (`self.swaySmoothFactor`))) false false))))))

(event `InputAxisKey|MouseY` :consume false
  (params (AxisValue :type "Float (single-precision)"))
  ;[1 1 1] Sway
  (goto _label))

(event `self.Fire`
  (bind _sk_richinnerlife (`self.SK_RichInnerLife`))
  (bind _sk_richinnerlife_2 (`self.SK_RichInnerLife`))
  ;[1 1 1] Fire
  (`GameplayStatics.SpawnEmitterAtLocation` "/Game/FX/Particles/Abilities/Ultimate/FX/P_TwinBlast_Ultimate_MuzzleFlash.P_TwinBlast_Ultimate_MuzzleFlash" (`SceneComponent.GetSocketLocation` _sk_richinnerlife "Muzzle") (`SceneComponent.GetSocketRotation` _sk_richinnerlife "Muzzle"))
  (`AudioComponent.Play` (`self.Audio`) 0.0)
  (`SceneComponent.K2_SetRelativeLocation` _sk_richinnerlife_2 (`KismetMathLibrary.VLerp` (`SceneComponent.RelativeLocation` _sk_richinnerlife_2) (+ (`KismetMathLibrary.MakeVector` -30.0) (`self.initialLocation`)) (* (`GameplayStatics.GetWorldDeltaSeconds`) 300.0)) false false))

(event `self.Equip`
  (bind _sk_richinnerlife (`self.SK_RichInnerLife`))
  ;[1 1 1] Equip
  (`SceneComponent.K2_SetRelativeLocation` (`self.SK_RichInnerLife`) (`self.holsteredLocation`) false false)
  (`Timeline|EquipTimeline`
    (:`Update`
      (`SceneComponent.K2_SetRelativeLocation` _sk_richinnerlife (`KismetMathLibrary.VLerp` (`SceneComponent.RelativeLocation` _sk_richinnerlife) (`self.initialLocation`) (* (`GameplayStatics.GetWorldDeltaSeconds`) (`self.equipSpeed`))) false false))
    (:`Finished`
      (`self.SetState` "NewEnumerator1"))))

(event `self.Unequip`
  (bind _sk_richinnerlife (`self.SK_RichInnerLife`))
  ;[1 1 1] Unequip
  (`Timeline|UnequipTimeline`
    (:`Update`
      (`SceneComponent.K2_SetRelativeLocation` _sk_richinnerlife (`KismetMathLibrary.VLerp` (`SceneComponent.RelativeLocation` _sk_richinnerlife) (`self.holsteredLocation`) (* (`GameplayStatics.GetWorldDeltaSeconds`) (`self.equipSpeed`))) false false))
    (:`Finished`
      (`self.SetState` "NewEnumerator4"))))

(fn `UserConstructionScript`
  (`parent.UserConstructionScript`)
  (set `self.initialLocation` (`SceneComponent.RelativeLocation` (`self.SK_RichInnerLife`)))
  (set `self.holsteredLocation` (- (`self.initialLocation`) (`self.holsterOffset`))))