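; Charge-and-release head gun, a child spawner Blueprint that launches BP_Ragdoll actors.
; Holding the trigger runs a timeline that builds Charge and head material brightness, with a Shepard-tone charge sound and a fully-charged cue.
; Releasing spawns a randomly rotated ragdoll at the arrow, passing Charge as Speed, then plays a burp and resets.
; Trigger state feeds the head's AnimBP; Fire is empty and the charge-pitch update is unwired.
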(event `self.ReceiveBeginPlay`
  ;[1 1 1] Setup
  (bind _asabp_head_gun (cast `/Game/GunJam/Guns/RagdollGun/RagdollGunRig/ABP_HeadGun` (`SkeletalMeshComponent.GetAnimInstance` (`self.Head`))))
  (set `self.AnimBPRef` _asabp_head_gun))

(event `self.Fire`)

(event `ResetChargeSound`
  (goto _label :!via `Reset`))

(event `self.PullTrigger`
  (bind _gunchargenoise (`self.GunChargeNoise`))
  ;[1 1 1] Pull trigger
  (set `/Game/GunJam/Guns/RagdollGun/RagdollGunRig/ABP_HeadGun.TriggerDown` true (`self.AnimBPRef`))
  (`|ExecutionSequence`
    (:`then_0`
      (`/Engine/EditorBlueprintResources/StandardMacros.DoOnce` false :!label _label
        (:`Completed`
          (bind _returnvalue (`GameplayStatics.SpawnSound2D` "/Game/GunJam/Guns/RagdollGun/RagdollGunRig/A_Shepard.A_Shepard" 1.2 (`KismetMathLibrary.RandomFloatInRange` 0.5 0.9) 0.0 null))
          (set `self.GunChargeNoise` _returnvalue))))
    (:`then_1`
      (bind (_direction _charge _gunmatbuildup _pitch) (`Timeline|SetCharge` :!via `PlayFromStart` :!label _label_2)
        (:`Update`
          (set `self.Charge` _charge)
          (`MaterialInstanceDynamic.SetScalarParameterValue` (`self.DynamicMatInst`) "Brightness" _gunmatbuildup)
          (`/Engine/EditorBlueprintResources/StandardMacros.IsValid` (`self.GunChargeNoise`)))
        (:`Finished`
          (`MaterialInstanceDynamic.SetScalarParameterValue` (`self.DynamicMatInst`) "Brightness" 10.0)
          (`/Engine/EditorBlueprintResources/StandardMacros.IsValid` _gunchargenoise
            (:`Is Valid`
              (`AudioComponent.Stop` _gunchargenoise))
            (:`Is Not Valid`
              _))
          (`GameplayStatics.PlaySound2D` "/Game/GunJam/Guns/RagdollGun/RagdollGunRig/A_FullyCharged.A_FullyCharged" 2.0 (`KismetMathLibrary.RandomFloatInRange` 0.85 1.2) 0.0 null null))))))

(event `self.ReleaseTrigger`
  (bind (_returnvalue_location _returnvalue_rotation) (`KismetMathLibrary.BreakTransform` (`self.GetTransform`)))
  (bind _gunchargenoise (`self.GunChargeNoise`))
  (bind (_returnvalue_x _returnvalue_y _returnvalue_z) (`KismetMathLibrary.BreakVector` (`SceneComponent.K2_GetComponentLocation` (`self.Arrow`))))
  ;[1 1 1] Release trigger
  (`|ExecutionSequence`
    (:`then_0`
      (goto _label_2 :!via `Stop`))
    (:`then_1`
      (`MaterialInstanceDynamic.SetScalarParameterValue` (`self.DynamicMatInst`) "Brightness" 0.0)
      (set `/Game/GunJam/Guns/RagdollGun/RagdollGunRig/ABP_HeadGun.TriggerDown` false (`self.AnimBPRef`))
      (bind _returnvalue (`|SpawnActorFromClass` "/Game/GunJam/Guns/RagdollGun/BP_Ragdoll.BP_Ragdoll_C" (`KismetMathLibrary.MakeTransform` (`KismetMathLibrary.MakeVector` _returnvalue_x _returnvalue_y (+ _returnvalue_z (`self.Offset`))) _returnvalue_rotation) "Undefined" "OverrideRootScale" null (`self.Charge`) null))
      (`SceneComponent.K2_SetRelativeRotation` (`/Game/GunJam/Guns/RagdollGun/BP_Ragdoll.Ragdoll` _returnvalue) (`KismetMathLibrary.MakeRotator` -90.0 (`KismetMathLibrary.RandomFloatInRange` 0.0 360.0) 90.0) false false)
      (set `self.Charge` 0.0))
    (:`then_2`
      (`/Engine/EditorBlueprintResources/StandardMacros.IsValid` _gunchargenoise
        (:`Is Valid`
          (`AudioComponent.Stop` _gunchargenoise))
        (:`Is Not Valid`
          _))
      (`GameplayStatics.PlaySound2D` "/Game/GunJam/Guns/RagdollGun/RagdollGunRig/A_Burp.A_Burp" 3.0 (`KismetMathLibrary.RandomFloatInRange` 0.6 1.6) 0.0 null null false)
      (`self.ResetChargeSound`))))

(fn `UserConstructionScript`
  (`parent.UserConstructionScript`)
  (bind _returnvalue (`PrimitiveComponent.CreateDynamicMaterialInstance` (`self.Head`) 0 "/Game/GunJam/Guns/RagdollGun/RagdollGunRig/M_HeadGun.M_HeadGun" "None"))
  (set `self.DynamicMatInst` _returnvalue))