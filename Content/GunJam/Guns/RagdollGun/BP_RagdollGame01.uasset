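; Ragdoll challenge zone that is won by keeping enough ragdolls inside its box for about ten seconds.
; Box overlaps count actors with "Ragdoll" in their name, updating the score text and a DoOnce-gated ticking sound.
; A looping timer fills the widget progress bar, resetting and pausing below target until ScoreCheck unpauses it.
; Completion destroys all BP_Ragdoll actors, shows the done text and plays an achievement sound.
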(event `self.ReceiveBeginPlay`
  (bind _returnvalue (`KismetSystemLibrary.K2_SetTimer` null "ScoreHolds" 1.0 true))
  (set `self.TimerHandler` _returnvalue)
  (bind _aswbp_score_holding_progress (cast `/Game/GunJam/Guns/RagdollGun/WBP_ScoreHoldingProgress` (`WidgetComponent.GetUserWidgetObject` (`self.Widget`))))
  (set `self.ProgressBarRef` _aswbp_score_holding_progress))

(event `self.Box.OnComponentBeginOverlap`
  (params (OverlappedComponent :type "PrimitiveComponent Object Reference") (OtherActor :type "Actor Object Reference") (OtherComp :type "PrimitiveComponent Object Reference") (OtherBodyIndex :type Integer) (bFromSweep :type Boolean) (SweepResult :type "HitResult Structure (by ref)"))
  (bind _score (`self.Score`))
  (if (and (`KismetStringLibrary.Contains` (`KismetStringLibrary.Conv_ObjectToString` OtherActor) "Ragdoll") (not (`self.ChallengeComplete`)))
    (`/Engine/EditorBlueprintResources/StandardMacros.IncrementInt` _score
      (:`  `
        (`self.ScoreCheck` _score :!label _label)
        (`self.ManageTickTockSound`)
        (`TextRenderComponent.K2_SetText` (`self.ScoreText`) (`KismetTextLibrary.Conv_IntToText` (`self.Score`)))))))

(event `self.Box.OnComponentEndOverlap`
  (params (OverlappedComponent :type "PrimitiveComponent Object Reference") (OtherActor :type "Actor Object Reference") (OtherComp :type "PrimitiveComponent Object Reference") (OtherBodyIndex :type Integer))
  (if (and (`KismetStringLibrary.Contains` (`KismetStringLibrary.Conv_ObjectToString` OtherActor) "Ragdoll") (not (`self.ChallengeComplete`)))
    (`/Engine/EditorBlueprintResources/StandardMacros.DecrementInt` (`self.Score`)
      (:`  `
        (goto _label)))))

(event `ManageTickTockSound`
  (bind _ticktocksound (`self.TickTockSound`))
  ;[1 1 1] tick tock sound
  (if (>= (`self.Score`) (`self.ScoreMax`))
    (`/Engine/EditorBlueprintResources/StandardMacros.DoOnce` false :!label _label_2
      (:`Completed`
        (bind _returnvalue (`GameplayStatics.SpawnSound2D` "/Game/GunJam/Guns/RagdollGun/TickTock.TickTock" 1.0 1.0 0.0 null))
        (set `self.TickTockSound` _returnvalue)))
    (else
      (`/Engine/EditorBlueprintResources/StandardMacros.IsValid` _ticktocksound
        (:`Is Valid`
          (`ActorComponent.K2_DestroyComponent` _ticktocksound)
          (goto _label_2 :!via `Reset`))))))

(fn `ScoreCheck`
  (params (Score :type Integer))
  (if (>= Score (`self.ScoreMax`))
    (`KismetSystemLibrary.K2_UnPauseTimerHandle` (`self.TimerHandler`))))

(fn `ScoreHolds`
  (bind _ticktocksound (`self.TickTockSound`))
  (if (>= (`self.Score`) (`self.ScoreMax`))
    (bind _result (`/Engine/EditorBlueprintResources/StandardMacros.IncrementInt` (`self.ScoreHoldsCheck`))
      (:`  `
        (if (>= _result 10)
          ;[1 1 1] Challenge completes
          (bind _outactors (`GameplayStatics.GetAllActorsOfClass` "/Game/GunJam/Guns/RagdollGun/BP_Ragdoll.BP_Ragdoll_C"))
          (`self.K2_DestroyActor` _outactors)
          (set `/Game/GunJam/Guns/RagdollGun/WBP_ScoreHoldingProgress.ProgressPercent` 1.0 (`self.ProgressBarRef`))
          (set `self.ChallengeComplete` true)
          (`SceneComponent.SetHiddenInGame` (`self.DoneText`) false false)
          (`SceneComponent.SetHiddenInGame` (`self.ScoreText`) true false)
          (`/Engine/EditorBlueprintResources/StandardMacros.IsValid` _ticktocksound
            (:`Is Valid`
              (`ActorComponent.K2_DestroyComponent` _ticktocksound))
            (:`Is Not Valid`
              _))
          (`GameplayStatics.PlaySound2D` "/Game/GunJam/Guns/RagdollGun/Ach.Ach" 1.0 1.0 0.0 null null)
          (else
            (set `/Game/GunJam/Guns/RagdollGun/WBP_ScoreHoldingProgress.ProgressPercent` (`KismetMathLibrary.MapRangeClamped` (`KismetMathLibrary.Conv_IntToDouble` (`self.ScoreHoldsCheck`)) 0.0 10.0 0.0 1.0) (`self.ProgressBarRef`))))))
    (else
      (set `self.ScoreHoldsCheck` 0)
      (`KismetSystemLibrary.K2_PauseTimerHandle` (`self.TimerHandler`))
      (set `/Game/GunJam/Guns/RagdollGun/WBP_ScoreHoldingProgress.ProgressPercent` 0.0 (`self.ProgressBarRef`)))))

(fn `UserConstructionScript`)