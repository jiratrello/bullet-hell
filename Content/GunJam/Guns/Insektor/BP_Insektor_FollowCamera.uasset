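; BP_Insektor_FollowCamera is a smoothed follow camera actor for the Insektor gun.
; It snaps to the target actor's CameraTarget component on BeginPlay.
; Each tick it eases toward that component with a lerp scaled by delta time and Factor, then rotates to look at the target actor's location.
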(event `self.ReceiveBeginPlay`
  (`self.K2_SetActorLocation` (`SceneComponent.K2_GetComponentLocation` (`/Game/GunJam/Guns/Insektor/BP_Insektor_Bug.CameraTarget` (`self.TargetActor`)))))

(event `self.ReceiveTick`
  (params (DeltaSeconds :type "Float (single-precision)"))
  (`|ExecutionSequence`
    (:`then_0`
      (`self.K2_SetActorLocation` (`KismetMathLibrary.VLerp` (`self.K2_GetActorLocation`) (`SceneComponent.K2_GetComponentLocation` (`/Game/GunJam/Guns/Insektor/BP_Insektor_Bug.CameraTarget` (`self.TargetActor`))) (* DeltaSeconds (`self.Factor`)))))
    (:`then_1`
      (`self.K2_SetActorRotation` (`KismetMathLibrary.FindLookAtRotation` (`self.K2_GetActorLocation`) (`self.K2_GetActorLocation` (`self.TargetActor`)))))))

(fn `UserConstructionScript`)