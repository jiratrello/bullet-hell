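; BP_Insektor_Bug is a player-steered flying bug pawn for the Insektor gun in GunJam.
; On BeginPlay, player controller 0 possesses it, then it spawns a BP_Insektor_FollowCamera targeting itself and blends the view to that camera.
; Tick pushes it constantly along its forward vector at Speed without sweeping, while the move axes feed controller yaw and pitch to steer; look axes are unused.
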(event `self.ReceiveBeginPlay`
  (`|ExecutionSequence`
    (:`then_0`
      (`Controller.Possess` (`GameplayStatics.GetPlayerController` 0) self))
    (:`then_1`
      (bind _returnvalue (`|SpawnActorFromClass` "/Game/GunJam/Guns/Insektor/BP_Insektor_FollowCamera.BP_Insektor_FollowCamera_C" (`self.GetTransform` self) "Undefined" "OverrideRootScale" null self null))
      (set `self.FollowCamera` _returnvalue)
      (`PlayerController.SetViewTargetWithBlend` (`GameplayStatics.GetPlayerController` 0) (`self.FollowCamera`) 1.0 "VTBlend_Linear" 0.0 false))))

(event `InputAxis|LookHorizontal`
  (params (AxisValue :type "Float (single-precision)")))

(event `InputAxis|MoveRight`
  (params (AxisValue :type "Float (single-precision)"))
  (`self.AddControllerYawInput` AxisValue))

(event `InputAxis|LookVertical`
  (params (AxisValue :type "Float (single-precision)")))

(event `InputAxis|MoveForward`
  (params (AxisValue :type "Float (single-precision)"))
  (`self.AddControllerPitchInput` AxisValue))

(event `self.ReceiveTick`
  (params (DeltaSeconds :type "Float (single-precision)"))
  (`self.K2_AddActorWorldOffset` (* (`KismetMathLibrary.GetForwardVector` (`self.K2_GetActorRotation` self)) (* DeltaSeconds (`self.Speed`)))))

(fn `UserConstructionScript`)