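; BP_Gun_Needler is an example Needler gun Blueprint that supplies the cosmetic response to Fire and Reload events.
; Fire plays a random sound from FireSounds, then restarts a recoil timeline that drives the GunNull component's X kickback and pitch rotation.
; Reload prints a debug string and plays the reload sound through the same audio component.
; No projectile, damage or ammo logic appears in this graph.
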(event `self.Fire`
  (`|ExecutionSequence`
    (:`then_0`
      ;[1 1 1] SFX
      (`AudioComponent.SetSound` (`self.Audio`) (`|GetArrayItem` (`self.FireSounds`) (`KismetMathLibrary.RandomInteger` (`KismetArrayLibrary.Array_Length` (`self.FireSounds`)))))
      (`AudioComponent.Play` (`self.Audio`) 0.0))
    (:`then_1`
      ;[1 1 1] Recoil Animation
      (bind (_direction _kickback _rotation) (`Timeline|RecoilAnimation` :!via `PlayFromStart`)
        (:`Update`
          (`SceneComponent.K2_SetRelativeLocation` (`self.GunNull`) (`KismetMathLibrary.MakeVector` _kickback) false false)
          (`SceneComponent.K2_SetRelativeRotation` (`self.GunNull`) (`KismetMathLibrary.MakeRotator` 0.0 _rotation) false false))))))

(event `self.Reload`
  (`KismetSystemLibrary.PrintString` "reloadd")
  (`AudioComponent.SetSound` (`self.Audio`) (`self.ReloadSound`))
  (`AudioComponent.Play` (`self.Audio`) 0.0))

(fn `UserConstructionScript`
  (`parent.UserConstructionScript`))