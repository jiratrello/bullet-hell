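; Spawner gun that places the selected entry from its Spawnables list at the aimed point, with right mouse cycling entries.
; Holding the trigger builds curve-scaled charge; releasing above the item's threshold spawns it with sparks and a flashbulb, optionally launching it by physics impulse.
; Tick sphere-traces to move a smoothed target indicator and drives charge, glow and motion-based animation into the WBP_Spawner widget, which also animates equip, unequip and firing.
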(event `Key|RightMouseButton`
  (params (Key :type "Key Structure"))
  (:`Pressed`
    (bind _result (`/Engine/EditorBlueprintResources/StandardMacros.IncrementInt` (`self.currentItemIndex`))
      (:`  `
        (bind _output_get (set `self.currentItemIndex` (mod _result (`KismetArrayLibrary.Array_Length` (`self.spawnables`)))))
        (set `self.currentItem` (`|GetArrayItem` (`self.spawnables`) _output_get))))))

(event `self.ReceiveBeginPlay`
  (bind _returnvalue (`|CreateWidget` "/Game/GunJam/Guns/Spawner/WBP_Spawner.WBP_Spawner_C"))
  (`UserWidget.AddToViewport` _returnvalue 0)
  (bind _output_get (set `self.UI` _returnvalue))
  (`/Game/GunJam/Guns/Spawner/WBP_Spawner.Setup` _output_get (`self.spawnables`))
  (set `self.currentItem` (`|GetArrayItem` (`self.spawnables`) (`self.currentItemIndex`))))

(event `self.ReceiveEndPlay`
  (params (EndPlayReason :type "EEndPlayReason Enum" :default "Destroyed"))
  (`Widget.RemoveFromParent` (`self.UI`))
  (`self.K2_DestroyActor` (`self.targetIndicator`)))

(event `self.PullTrigger`
  (set `self.held` true)
  (`AudioComponent.Play` (`self.AudioCharge`) 0.0)
  (`AudioComponent.Play` (`self.AudioHoldingCharge`) 0.0))

(event `self.ReleaseTrigger`
  (bind _currentitem_chargelevel (break `/Game/GunJam/Guns/Spawner/SpawnItemData` (`self.currentItem`)))
  (bind _ui (`self.UI`))
  (`|ExecutionSequence`
    (:`then_0`
      (bind (_outhit _returnvalue) (`self.Trace`))
      (if _returnvalue
        (if (>= (`self.charge`) _currentitem_chargelevel)
          (`self.SpawnSpawnable` (`self.currentItem`) (`SceneComponent.K2_GetComponentLocation` (`self.DefaultSceneRoot`)) (`.Location` (`GameplayStatics.BreakHitResult` _outhit)))
          (`UserWidget.PlayAnimation` _ui (`/Game/GunJam/Guns/Spawner/WBP_Spawner.Shoot` _ui) 0.0 1 "Forward" 1.0 false)
          (set `self.glowAmount` 1.0)
          (`AudioComponent.Play` (`self.AudioFire`) 0.0))))
    (:`then_1`
      (set `self.held` false)
      (set `/Game/GunJam/Guns/Spawner/WBP_Spawner.charge` 0.0 (`self.UI`))
      (set `self.charge` 0.0))
    (:`then_2`
      (`AudioComponent.Stop` (`self.AudioCharge`))
      (`AudioComponent.Stop` (`self.AudioHoldingCharge`)))))

(event `self.ReceiveTick`
  (params (DeltaSeconds :type "Float (single-precision)"))
  (`|ExecutionSequence`
    (:`then_0`
      (`self.UpdateCharge` DeltaSeconds))
    (:`then_1`
      (`self.UpdateMaterialParameters`))
    (:`then_2`
      (`self.UpdateAnimationSpeed` DeltaSeconds))
    (:`then_3`
      (`self.UpdateGlow` DeltaSeconds))))

(event `self.Equip`
  (bind _ui (`self.UI`))
  (bind _enter (`/Game/GunJam/Guns/Spawner/WBP_Spawner.Enter` _ui))
  (`UserWidget.PlayAnimation` _ui _enter 0.0 1 "Forward" 1.0 false)
  (`KismetSystemLibrary.Delay` (`WidgetAnimation.GetEndTime` _enter))
  (`self.SetState` "NewEnumerator1"))

(event `self.Unequip`
  (bind _ui (`self.UI`))
  (bind _exit (`/Game/GunJam/Guns/Spawner/WBP_Spawner.Exit` _ui))
  (`UserWidget.PlayAnimation` _ui _exit 0.0 1 "Forward" 1.0 false)
  (`KismetSystemLibrary.Delay` (`WidgetAnimation.GetEndTime` _exit))
  (`self.SetState` "NewEnumerator4"))

(fn `Get Spawnable`
  (returns (ChargeLevel :type "/Game/GunJam/Guns/Spawner/SpawnItemData Structure") (success :type Boolean))
  (locals (spawnCandidate :type "/Game/GunJam/Guns/Spawner/SpawnItemData Structure") (yay :type Boolean))
  (for _array_element (`self.spawnables`)
    (if (> (`self.charge`) (`.chargeLevel_2_AEA64C50410A159B41DAE4A1F03A6FAE` (break `/Game/GunJam/Guns/Spawner/SpawnItemData` _array_element)))
      (set `local.spawnCandidate` _array_element)
      (set `local.yay` true)
      (else
        (break))))
  (return (`local.spawnCandidate`) (`local.yay`)))

(fn `SpawnSpawnable`
  (params (toSpawn :type "/Game/GunJam/Guns/Spawner/SpawnItemData Structure") (startPosition :type "Vector Structure") (endPosition :type "Vector Structure"))
  (locals (direction :type "Vector Structure" :default (0.0 0.0 0.0)) (spawnLocation :type "Vector Structure"))
  (bind _direction (`local.direction`))
  (set `local.direction` (- endPosition startPosition))
  (bind _output_get (set `local.spawnLocation` (select `bool` toSpawn_shootPhysics_14_71DEED234A9FC0B629F5FE82B35898D8 :`false` endPosition :`true` (`KismetMathLibrary.VLerp` startPosition endPosition 0.9))))
  (bind _returnvalue (`|SpawnActorFromClass` toSpawn_actorToSpawn_6_71D569DA4B43A014D0AE9D9DE4E1C758 (`KismetMathLibrary.MakeTransform` _output_get (select `bool` toSpawn_randomRotation_11_FBC8634F43632C6C4BCCC08885B59680 :`true` (`KismetMathLibrary.RandomRotator` true))) "Undefined" "OverrideRootScale" null null))
  (`GameplayStatics.SpawnEmitterAtLocation` "/Game/GunJam/Guns/Spawner/Things/SparksParticle.SparksParticle" (`local.spawnLocation`))
  (`|SpawnActorFromClass` "/Game/GunJam/Guns/Spawner/Things/BP_Flashbulb.BP_Flashbulb_C" (`KismetMathLibrary.MakeTransform` (`local.spawnLocation`)) "Undefined" "OverrideRootScale" null null)
  ;[1 1 1] physics impulse
  (if toSpawn_shootPhysics_14_71DEED234A9FC0B629F5FE82B35898D8
    (for _array_element (`self.K2_GetComponentsByClass` _returnvalue "/Script/Engine.StaticMeshComponent")
      (`PrimitiveComponent.AddImpulse` _array_element (* (`KismetMathLibrary.Normal` _direction) (`KismetMathLibrary.MapRangeClamped` (`KismetMathLibrary.VSize` _direction) 0.0 1000.0 1000.0 3000.0)) "None" false))))

(fn `Trace`
  (returns (OutHit :type "HitResult Structure") (ReturnValue :type Boolean))
  (locals (localHit :type "HitResult Structure"))
  (bind _defaultsceneroot (`self.DefaultSceneRoot`))
  (bind _returnvalue (`SceneComponent.K2_GetComponentLocation` _defaultsceneroot))
  (bind (_outhit _returnvalue_2) (`KismetSystemLibrary.SphereTraceSingleForObjects` :`Start` _returnvalue :`End` (+ _returnvalue (* (`KismetMathLibrary.GetForwardVector` (`SceneComponent.K2_GetComponentRotation` _defaultsceneroot)) 2000.0)) :`Radius` 10.0 :`ObjectTypes` (`|MakeArray` "ObjectTypeQuery1" "ObjectTypeQuery4" "ObjectTypeQuery2" :!type "EObjectTypeQuery Enum") :`DrawTime` 0.5))
  (`self.UpdateTarget` _outhit _returnvalue_2)
  (return _outhit _returnvalue_2))

(fn `UpdateAnimationSpeed`
  (params (delta :type "Float (double-precision)"))
  (if (> (`KismetMathLibrary.VSize` (- (`SceneComponent.K2_GetComponentLocation` (`self.DefaultSceneRoot`)) (`self.lastPosition`))) 1.0)
    (set `self.animationSpeed` (`KismetMathLibrary.FClamp` (+ (`self.animationSpeed`) (* delta 3.0))))
    (else
      (set `self.animationSpeed` (* (`self.animationSpeed`) 0.95))))
  (`/Game/GunJam/Guns/Spawner/WBP_Spawner.SetAnimationSpeed` (`self.UI`) (`self.animationSpeed`))
  (set `self.lastPosition` (`SceneComponent.K2_GetComponentLocation` (`self.DefaultSceneRoot`))))

(fn `UpdateCharge`
  (params (A :type "Float (double-precision)"))
  (bind (_currentitem_chargelevel _currentitem_actortospawn _currentitem_title) (break `/Game/GunJam/Guns/Spawner/SpawnItemData` (`self.currentItem`)))
  (bind _currentitem_chargelevel_2 (break `/Game/GunJam/Guns/Spawner/SpawnItemData` (`self.currentItem`)))
  (set `/Game/GunJam/Guns/Spawner/WBP_Spawner.title` _currentitem_title (`self.UI`))
  (`self.Trace`)
  (if (`self.held`)
    (bind _output_get (set `self.charge` (+ (* A (* (`self.baseChargeRate`) (`CurveFloat.GetFloatValue` (`self.chargeCurve`) (`self.charge`)))) (`self.charge`))))
    (set `/Game/GunJam/Guns/Spawner/WBP_Spawner.charge` (`KismetMathLibrary.FClamp` (/ _output_get _currentitem_chargelevel_2)) (`self.UI`))))

(fn `UpdateGlow`
  (params (delta :type "Float (double-precision)"))
  (bind _output_get (set `self.glowAmount` (`KismetMathLibrary.FClamp` (- (`self.glowAmount`) (* delta 0.5)))))
  (`LightComponent.SetIntensity` (`self.PointLight`) (* (`KismetMathLibrary.FClamp` (- _output_get 0.7)) 10000.0)))

(fn `UpdateMaterialParameters`
  (`/Game/GunJam/Guns/Spawner/WBP_Spawner.SetViewDirection` (`self.UI`) (`KismetMathLibrary.InverseTransformDirection` (`self.GetTransform`) (`KismetMathLibrary.Normal` (0.3 0.2 1.0))))
  (`/Game/GunJam/Guns/Spawner/WBP_Spawner.SetGlowAmount` (`self.UI`) (`self.glowAmount`)))

(fn `UpdateTarget`
  (params (hit :type "HitResult Structure") (result :type Boolean))
  (bind (_hit_bblockinghit _hit_binitialoverlap _hit_time _hit_distance _hit_location _hit_impactpoint _hit_normal) (`GameplayStatics.BreakHitResult` (`local.hit`)))
  (bind _targetindicator (`self.targetIndicator`))
  (bind _targetindicator_2 (`self.targetIndicator`))
  (if result
    (`|ExecutionSequence`
      (:`then_0`
        (`/Engine/EditorBlueprintResources/StandardMacros.IsValid` (`self.targetIndicator`)
          (:`Is Not Valid`
            (bind _returnvalue (`|SpawnActorFromClass` "/Game/GunJam/Guns/Spawner/BP_SpawnerTarget.BP_SpawnerTarget_C" (`KismetMathLibrary.MakeTransform` (0.0 0.0 0.0)) "Undefined" "OverrideRootScale" null null))
            (set `self.targetIndicator` _returnvalue))))
      (:`then_1`
        (`self.K2_SetActorLocation` _targetindicator (`KismetMathLibrary.VLerp` (`self.K2_GetActorLocation` _targetindicator) _hit_location 0.3) false false))
      (:`then_2`
        (`self.K2_SetActorRotation` (`self.targetIndicator`) (`KismetMathLibrary.Conv_VectorToRotator` _hit_normal) false)))
    (else
      (`/Engine/EditorBlueprintResources/StandardMacros.IsValid` _targetindicator_2
        (:`Is Valid`
          (`self.K2_DestroyActor` _targetindicator_2))))))

(fn `UserConstructionScript`
  (`parent.UserConstructionScript`))