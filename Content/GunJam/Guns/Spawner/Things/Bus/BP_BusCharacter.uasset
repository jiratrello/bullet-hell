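; BP_BusCharacter is a bus character that wanders between random nearby goals on the ground plane.
; NewGoal picks a grid-stepped offset from its location and resets a random boredom timer; Tick picks another when the timer expires or the goal is close.
; Tick feeds UpdateMoveVector into slow movement input and draws a debug sphere at the goal.
; The goal-steering lerp inside UpdateMoveVector is left unconnected.
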(event `self.ReceiveBeginPlay`
  (`self.NewGoal`))

(event `self.ReceiveTick`
  (params (DeltaSeconds :type "Float (single-precision)"))
  (bind _returnvalue (`KismetMathLibrary.VLerp` (`self.MoveVector`) (`KismetMathLibrary.Normal` (- (`self.GoalPosition`) (`SceneComponent.K2_GetComponentLocation` (`self.CapsuleComponent`))) 1e-06) (* DeltaSeconds 3.0)))
  (set `self.BoredTimer` (- (`self.BoredTimer`) DeltaSeconds))
  (`KismetSystemLibrary.DrawDebugSphere` (`self.GoalPosition`) 30.0 12 (struct :`R` 1.0 :`B` 0.478248 :`A` 1.0))
  (set `self.MoveVector` (`KismetMathLibrary.VLerp` _returnvalue (`KismetMathLibrary.Normal` _returnvalue) 0.1))
  (`self.AddMovementInput` (`self.MoveVector`) 0.3)
  (if (<= (`self.BoredTimer`) 0.0)
    (`self.NewGoal` :!label _label)
    (elif (< (`KismetMathLibrary.VSize` (- (`self.GoalPosition`) (`SceneComponent.K2_GetComponentLocation` (`self.CapsuleComponent`)))) 50.0)
      (goto _label))))

(fn `NewGoal`
  (set `self.GoalPosition` (+ (`SceneComponent.K2_GetComponentLocation` (`self.CapsuleComponent`)) (`KismetMathLibrary.MakeVector` (* (`KismetMathLibrary.RandomIntegerInRange` -3 3) 100.0) (* (`KismetMathLibrary.RandomIntegerInRange` -3 3) 100.0))))
  (set `self.BoredTimer` (`KismetMathLibrary.RandomFloatInRange` 3.0 4.0)))

(fn `UserConstructionScript`)