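; BP_Flashbulb is a short-lived actor that produces a flash of light which quickly fades out.
; BeginPlay records the point light's starting intensity.
; Tick advances a clamped alpha at a fixed rate, fading the light linearly to zero in about a fifth of a second, then destroys the actor.
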(event `self.ReceiveBeginPlay`
  (set `self.initialBright` (`LightComponentBase.Intensity` (`self.PointLight`))))

(event `self.ReceiveTick`
  (params (DeltaSeconds :type "Float (single-precision)"))
  (set `self.lerp` (`KismetMathLibrary.FClamp` (+ (`self.lerp`) (* DeltaSeconds 5.0))))
  (`LightComponent.SetIntensity` (`self.PointLight`) (`KismetMathLibrary.Lerp` (`self.initialBright`) 0.0 (`self.lerp`)))
  (if (>= (`self.lerp`) 1.0)
    (`self.K2_DestroyActor`)))

(fn `UserConstructionScript`)