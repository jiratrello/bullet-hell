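; BP_Gun_Vito is a tendril gun that winds up while the trigger is held and fires BP_VitoBullet projectiles.
; Tick raises a capped FiringSpeed, prints it and feeds it to ABP_TendrilGun as a fire speed multiplier, while releasing the trigger resets it.
; AnimationFired spawns each bullet from alternating Flower1 and Flower2 transforms, passing the raw FiringSpeed to its AddImpulse, as the range remap is unused.
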(event `self.ReceiveTick`
  (params (DeltaSeconds :type "Float (single-precision)"))
  (if (`self.TriggerHeld`)
    (bind _output_get (set `self.FiringSpeed` (`KismetMathLibrary.FMin` (+ (`self.FiringSpeed`) DeltaSeconds) 6.0)))
    (`KismetSystemLibrary.PrintString` (`KismetStringLibrary.Conv_DoubleToString` _output_get) true true (struct :`G` 0.66 :`B` 1.0 :`A` 1.0) 2.0 "fireSpeed")
    (set `/Game/GunJam/Guns/Vito/VitoGun/ABP_TendrilGun.FireSpeedMultiplier` _output_get (`self.ABPTendrils`))))

(event `self.ReceiveBeginPlay`
  (bind _returnvalue (`SkeletalMeshComponent.GetAnimInstance` (`self.Tendrils`)))
  (`/Engine/EditorBlueprintResources/StandardMacros.IsValid` _returnvalue
    (:`Is Valid`
      (bind _asabp_tendril_gun (cast `/Game/GunJam/Guns/Vito/VitoGun/ABP_TendrilGun` _returnvalue))
      (set `self.ABPTendrils` _asabp_tendril_gun))))

(event `self.PullTrigger`
  (set `/Game/GunJam/Guns/Vito/VitoGun/ABP_TendrilGun.Firing` true (`self.ABPTendrils`))
  (set `self.TriggerHeld` true))

(event `self.ReleaseTrigger`
  (set `/Game/GunJam/Guns/Vito/VitoGun/ABP_TendrilGun.Firing` false (`self.ABPTendrils`))
  (set `self.TriggerHeld` false)
  (set `self.FiringSpeed` 0.5))

(event `AnimationFired`
  (bind _returnvalue (`|SpawnActorFromClass` "/Game/GunJam/Guns/Vito/BP_VitoBullet.BP_VitoBullet_C" (`SceneComponent.K2_GetComponentToWorld` (select `bool` (`self.flowerToggle`) :`false` (`self.Flower1`) :`true` (`self.Flower2`))) "Undefined" "OverrideRootScale" null null))
  (`/Game/GunJam/Guns/Vito/BP_VitoBullet.AddImpulse` _returnvalue (`self.FiringSpeed`))
  (set `self.flowerToggle` (not (`self.flowerToggle`))))

(fn `UserConstructionScript`
  (`parent.UserConstructionScript`))