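; Projectile actor for the Vito gun, a bullet moved by a physics impulse.
; The AddImpulse event pushes the static mesh along the actor's forward vector, scaled by the supplied Force.
; Tick counts LifeTime down and destroys the actor once it drops below zero.
; The graph contains no hit or damage logic.
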(event `AddImpulse`
  (params (Force :type "Float (double-precision)"))
  (`PrimitiveComponent.AddImpulse` (`self.StaticMesh`) (* (`self.GetActorForwardVector`) Force) "None" false))

(event `self.ReceiveTick`
  (params (DeltaSeconds :type "Float (single-precision)"))
  (bind _output_get (set `self.LifeTime` (- (`self.LifeTime`) DeltaSeconds)))
  (if (< _output_get 0.0)
    (`self.K2_DestroyActor`)))

(fn `UserConstructionScript`)